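; Sliding tile puzzle actor with mouse and touch input, sized from 2x2 to 5x5.
; The construction script builds a centered grid of mesh blocks, slices the image across them via dynamic materials, hides the last as the blank and shuffles by preset seed or randomly, which may be unsolvable.
; Clicked blocks found by a sphere overlap around the blank slide into it.
; Matching the saved goal array reveals the blank, unbinds input and prints a finish message.
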(event `self.ReceiveBeginPlay`
  ;[0 0 0] Loop for each Puzzle Block that is visible (excluding the blank one)
  (for _array_element (`self.PuzzleBlocks`)
    (if (`SceneComponent.IsVisible` _array_element)
      ;[0 0 0] Mouse Click Support
      (add `PrimitiveComponent.OnClicked` _array_element (`|CreateDelegate` :!event `Block Clicked`))
      ;[0 0 0] Mobile Support
      (add `PrimitiveComponent.OnInputTouchEnd` _array_element (`|CreateDelegate` :!event `Block Touched`)))))

(event `Block Clicked`
  (params (TouchedComponent :type "PrimitiveComponent Object Reference") (ButtonPressed :type "Key Structure" :default "None"))
  ;[0 0 0] Block Clicked by Mouse
  (if (not (`self.Delay`))
    (set `self.SelectedBlock` (cast `StaticMeshComponent` TouchedComponent :!pure true))
    ;[0 0 0] Focus to the puzzle
    (`WidgetBlueprintLibrary.SetInputMode_GameAndUIEx` (`GameplayStatics.GetPlayerController` 0) null :!label _label)
    ;[0 0 0] Sphere Trace from the blank block.
    (bind (_outcomponents _returnvalue) (`KismetSystemLibrary.SphereOverlapComponents` (`SceneComponent.K2_GetComponentLocation` (`self.BlankBlock`)) (* (* (`self.MeshWidth`) (/ (/ (`self.PuzzleWidth`) (`KismetMathLibrary.Conv_IntToDouble` (`self.PuzzleSize`))) (`self.MeshWidth`))) 0.7) (`|MakeArray` "ObjectTypeQuery2" :!type "EObjectTypeQuery Enum") "/Script/Engine.StaticMeshComponent"))
    ;[0 0 0] Check whether the clicked block is near the blank block if the hit result is true.
    (if _returnvalue
      (for _array_element _outcomponents
        (if (== _array_element (`self.SelectedBlock`))
          ;[0 0 0] Set Delay to true, so you can't move another block while the last clicked block is moving.
          (set `self.Delay` true)
          ;[0 0 0] Swap the clicked block with the blank one.
          (`KismetArrayLibrary.Array_Swap` (`self.PuzzleBlocks`) (`KismetArrayLibrary.Array_Find` (`self.PuzzleBlocks`) (`self.SelectedBlock`)) (`KismetArrayLibrary.Array_Find` (`self.PuzzleBlocks`) (`self.BlankBlock`)))
          ;[0 0 0] Play Click Sound if you want.
          (`GameplayStatics.PlaySoundAtLocation` (`self.ClickSound`) (`self.K2_GetActorLocation`) (struct) 2.0 1.0 0.0 null null null)
          ;[0 0 0] Moving the Clicked Block to the blank position.
          (`KismetSystemLibrary.MoveComponentTo` (`self.SelectedBlock`) (`|GetArrayItem` (`self.PuzzleLocations`) (`KismetArrayLibrary.Array_Find` (`self.PuzzleBlocks`) (`self.SelectedBlock`))) (struct) true true (`self.MoveSpeed`) true)
          ;[0 0 0] After moving, just set the blank one to the last position of the clicked block.
          (`SceneComponent.K2_SetRelativeLocation` (`self.BlankBlock`) (`|GetArrayItem` (`self.PuzzleLocations`) (`KismetArrayLibrary.Array_Find` (`self.PuzzleBlocks`) (`self.BlankBlock`))) false false)
          ;[0 0 0] End Delay, now you can execute your next move.
          (set `self.Delay` false)
          ;[0 0 0] Now, check if we finished the puzzle.
          (if (`KismetArrayLibrary.Array_Identical` (`self.PuzzleBlocks`) (`self.PuzzleGoal`))
            ;[0 0 0] If true, visible the blank one.
            (`SceneComponent.SetVisibility` (`self.BlankBlock`) true true)
            ;[0 0 0] Unbind all click events.
            (for _array_element_2 (`self.PuzzleBlocks`)
              (if (`SceneComponent.IsVisible` _array_element_2)
                (remove `PrimitiveComponent.OnClicked` _array_element_2 (`|CreateDelegate` :!event `Block Clicked`))
                (remove `PrimitiveComponent.OnInputTouchEnd` _array_element_2 (`|CreateDelegate` :!event `Block Touched`))))
            ;[0 0 0] Add your finishment visual feedback here.
            (`KismetSystemLibrary.PrintString` "FINISHED!!!" true false (struct :`G` 1.0 :`A` 1.0) 5.0)))))))

(event `Block Touched`
  (params (FingerIndex :type "ETouchIndex Enum" :default "Touch1") (TouchedComponent :type "PrimitiveComponent Object Reference"))
  ;[0 0 0] Block Touched by Finger
  (if (not (`self.Delay`))
    (set `self.SelectedBlock` (cast `StaticMeshComponent` TouchedComponent :!pure true))
    (goto _label)))

(fn `BlockGeneration`
  (bind _puzzleblocks (`self.PuzzleBlocks`))
  (bind _spring_arm (`self.Spring Arm`))
  (bind _puzzleblocks_2 (`self.PuzzleBlocks`))
  (bind _returnvalue (/ 1.0 (`KismetMathLibrary.Conv_IntToDouble` (`self.PuzzleSize`))))
  (bind _returnvalue_2 (/ (`self.PuzzleWidth`) (`KismetMathLibrary.Conv_IntToDouble` (`self.PuzzleSize`))))
  (bind _returnvalue_3 (/ _returnvalue_2 (`self.MeshWidth`)))
  (bind _returnvalue_4 (* (/ (- (`self.PuzzleWidth`) (* (`self.MeshWidth`) (/ (/ (`self.PuzzleWidth`) (`KismetMathLibrary.Conv_IntToDouble` (`self.PuzzleSize`))) (`self.MeshWidth`)))) 2.0) -1.0))
  ;[0 0 0] Destroy and Clean the Last Generated Blocks, otherwise the construction script will generate the blocks each time you update the custom variable of your puzzle instance in the scene.
  (for _array_element (`self.PuzzleBlocks`)
    (`ActorComponent.K2_DestroyComponent` _array_element))
  (`KismetArrayLibrary.Array_Clear` (`self.PuzzleBlocks`))
  ;[0 0 0] Restore the size of the puzzle, which represents the number of cells in the vertical and horizontal direction of it. You can add more options to the enum named Puzzle Division, and then fill the Select Node with corresponding value.
  (set `self.PuzzleSize` (select `/Game/MiniGamePack_SlidingPuzzle/Blueprints/Enum_PuzzleDivision` (`self.PuzzleDivision`) :`NewEnumerator2` 2 :`NewEnumerator0` 3 :`NewEnumerator1` 4 :`NewEnumerator3` 5))
  ;[0 0 0] This loop controls the Generation Row, the output index means which row is now generating.
  (for _index (range (`self.PuzzleSize`))
    (set `self.GenerationYIndex` _index)
    ;[0 0 0] This loop will spawn each puzzle block in the current Row, the output index means which block in this row is now spawning. Once the generaction in current row finished, then the previous loop will start a new row, and the index value in this loop will back to 0.
    (for _index_2 (range (`self.PuzzleSize`))
      (set `self.GenerationXIndex` _index_2)
      ;[0 0 0] Add a Block to the Scene Component named Blocks, and initialize the relative location according to its Horizontal and vertical index as well as its 3D scale value. The Position and Sacle will be affected by custom puzzle width and thickness. The meaning of those custom variables is in the tooltip description.
      (bind _returnvalue_5 (`AddComponent|NODE_AddStaticMeshComponent-1` :`bManualAttachment` true :`RelativeTransform` (`KismetMathLibrary.MakeTransform` (`KismetMathLibrary.MakeVector` (* (`self.GenerationXIndex`) _returnvalue_2) (* (`self.GenerationYIndex`) _returnvalue_2)) (struct) (`KismetMathLibrary.MakeVector` _returnvalue_3 _returnvalue_3 (`self.PuzzleThickness`)))))
      ;[0 0 0] Save the Block to the array. This array contains all the puzzle blocks including the transparent one (the last index of the current size grid).
      (`KismetArrayLibrary.Array_Add` (`self.PuzzleBlocks`) _returnvalue_5)
      ;[0 0 0] Attach the block to the Scene Component named Blocks, and then we will use the component to center the whole puzzle.
      (`SceneComponent.K2_AttachToComponent` _returnvalue_5 (`self.Blocks`) "None" "KeepRelative" "KeepRelative" "KeepRelative" true)
      ;[0 0 0] Set material for the sides of the mesh
      (`PrimitiveComponent.SetMaterial` _returnvalue_5 1 "/Engine/BasicShapes/BasicShapeMaterial.BasicShapeMaterial")
      ;[0 0 0] Create the MID to handle the texture of each puzzle block.
      (bind _returnvalue_6 (`PrimitiveComponent.CreateDynamicMaterialInstance` _returnvalue_5 0 "/Game/MiniGamePack_SlidingPuzzle/Materials/MI_SlidingPuzzle.MI_SlidingPuzzle" "None"))
      ;[0 0 0] Handle Puzzle Texture (Image). Set the texture for all blocks with your custom image if you have customized it in the variable called Puzzle Image.
      (`MaterialInstanceDynamic.SetTextureParameterValue` _returnvalue_6 "Puzzle Texture" (select `bool` (`KismetSystemLibrary.IsValid` (`self.PuzzleImage`)) :`false` (select `/Game/MiniGamePack_SlidingPuzzle/Blueprints/Enum_PuzzleDivision` (`self.PuzzleDivision`) :`NewEnumerator2` "/Game/MiniGamePack_SlidingPuzzle/Textures/T_SlidingPuzzle_Gird_2x2.T_SlidingPuzzle_Gird_2x2" :`NewEnumerator0` "/Game/MiniGamePack_SlidingPuzzle/Textures/T_SlidingPuzzle_Gird_3x3.T_SlidingPuzzle_Gird_3x3" :`NewEnumerator1` "/Game/MiniGamePack_SlidingPuzzle/Textures/T_SlidingPuzzle_Gird_4x4.T_SlidingPuzzle_Gird_4x4" :`NewEnumerator3` "/Game/MiniGamePack_SlidingPuzzle/Textures/T_SlidingPuzzle_Gird_5x5.T_SlidingPuzzle_Gird_5x5" :!type "Texture Object Reference") :`true` (`self.PuzzleImage`)))
      ;[0 0 0] Passing in the Puzzle Subsection Parameter to the MID.
      (`MaterialInstanceDynamic.SetScalarParameterValue` _returnvalue_6 "Size" (`KismetMathLibrary.Conv_IntToDouble` (`self.PuzzleSize`)))
      ;[0 0 0] Cut the picture into pieces, then choose the correct Texture part to fill the block.
      (`MaterialInstanceDynamic.SetScalarParameterValue` _returnvalue_6 "X" (* (`KismetMathLibrary.Conv_IntToDouble` (`self.GenerationXIndex`)) _returnvalue))
      (`MaterialInstanceDynamic.SetScalarParameterValue` _returnvalue_6 "Y" (* _returnvalue (`KismetMathLibrary.Conv_IntToDouble` (`self.GenerationYIndex`))))))
  ;[0 0 0] Set the block of the last index to invisible, so it will be a ‘blank’ that nearby blocks can move to.
  (bind _output_get (set `self.BlankBlock` (`|GetArrayItem` _puzzleblocks_2 (`KismetArrayLibrary.Array_LastIndex` _puzzleblocks_2))))
  (`SceneComponent.SetVisibility` _output_get false false)
  ;[0 0 0] Center the puzzle to the coordinate axis, then we can move and rotate the puzzle blueprint in the map scene easily.
  (`SceneComponent.K2_SetRelativeLocation` (`self.Blocks`) (`KismetMathLibrary.MakeVector` _returnvalue_4 _returnvalue_4) false false)
  ;[0 0 0] After the generation, the layout of all blocks is the goal we need to reach. Then we will shuffle the puzzle blocks or move them to the new position, so this saved array will help we to check if we have finished the puzzle.
  (set `self.PuzzleGoal` (`self.PuzzleBlocks`))
  ;[0 0 0] Controls the Spring Arm of the Camera of the puzzle.
  (set `SpringArmComponent.TargetArmLength` (`self.SpringArmLength`) _spring_arm)
  (`SceneComponent.K2_SetRelativeRotation` _spring_arm (`KismetMathLibrary.MakeRotator` 0.0 (`self.SpringArmPitch`) -90.0) false false)
  ;[0 0 0] Restore the relative positions of all puzzle blocks (including that blank block) and save them into the position array.
  (for _array_element_2 (`self.PuzzleBlocks`)
    (`KismetArrayLibrary.Array_Add` (`self.PuzzleLocations`) (`SceneComponent.RelativeLocation` _array_element_2)))
  ;[0 0 0] The last step, you can determine whether the puzzle blocks need to shuffle, if yes you can enable seed shuffle mode.
  (if (`self.Shuffle`)
    (if (`self.UseSeed`)
      ;[0 0 0] If yes, then use the seed data to arrange the blocks. The Data in the Seed is recorded once I tried and successfully completed the puzzle without any bugs, if you try to not use the seed and shuffle it randomly, sometimes the bug will happen, so you can try and find new seed and record it to a new variable.
      (for (_ _array_index) (`self.PuzzleBlocks`)
        (`KismetArrayLibrary.Array_Set` (`self.PuzzleBlocks`) _array_index (`|GetArrayItem` (`self.PuzzleGoal`) (- (`|GetArrayItem` (select `/Game/MiniGamePack_SlidingPuzzle/Blueprints/Enum_PuzzleDivision` (`self.PuzzleDivision`) :`NewEnumerator2` (`|MakeArray` 2 3 4 1) :`NewEnumerator0` (select `int` (`self.SeedIndex`) :`0` (`self.Seed 3x3 A`) :`1` (`self.Seed 3x3 B`) :`2` (`self.Seed 3x3 C`) :`3` (`self.Seed 3x3 D`)) :`NewEnumerator1` (select `int` (`self.SeedIndex`) :`0` (`self.Seed 4x4 A`) :`1` (`self.Seed 4x4 B`) :`2` (`self.Seed 4x4 C`) :`3` (`self.Seed 4x4 D`)) :`NewEnumerator3` (select `int` (`self.SeedIndex`) :`0` (`self.Seed 5x5 A`) :`1` (`self.Seed 5x5 B`) :`2` (`self.Seed 5x5 C`) :`3` (`self.Seed 5x5 D`))) _array_index) 1)) true))
      (else
        ;[0 0 0] If you don't wanna use the seed to shuffle, then just shuffle it randomly and then move the blank block to the last index of the array. But you may come across with the bug that the puzzle can't be finished.
        (`KismetArrayLibrary.Array_Shuffle` _puzzleblocks)
        (`KismetArrayLibrary.Array_Swap` _puzzleblocks (`KismetArrayLibrary.Array_Find` (`self.PuzzleBlocks`) (`self.BlankBlock`)) (`KismetArrayLibrary.Array_LastIndex` (`self.PuzzleBlocks`)))))
    ;[0 0 0] Last step, place each puzzle block in its corresponding position.
    (for (_array_element_3 _array_index_2) (`self.PuzzleBlocks`)
      (`SceneComponent.K2_SetRelativeLocation` _array_element_3 (`|GetArrayItem` (`self.PuzzleLocations`) _array_index_2) false false))))

(fn `UserConstructionScript`
  ;[1 1 1] Generation
  (`self.BlockGeneration`) ; Generate all puzzle blocksw with custom parameters.
)