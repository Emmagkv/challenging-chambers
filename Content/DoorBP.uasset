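; Door Blueprint that swings its static mesh open once enough triggers have called Open.
; Each Open call increments a counter, and reaching the TriggerNumbers threshold plays a timeline that lerps the mesh's relative rotation to 90 degrees.
; Close reverses that timeline without resetting the counter.
; The door sound fires as a 2D sound on every timeline update, so it retriggers throughout movement in either direction.
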(event `Open`
  (params (trigger :type "/Game/Puzzletrigger Object Reference"))
  (bind _result (`/Engine/EditorBlueprintResources/StandardMacros.IncrementInt` (`self.countingtriggers`))
    (:`  `
      (if (>= _result (`self.TriggerNumbers`))
        (bind (_direction _track) (`Timeline|TL_open` :!label _label)
          (:`Update`
            (`GameplayStatics.PlaySound2D` "/Game/Sounds/door-43633_Cue.door-43633_Cue" 1.0 1.0 0.0 null null)
            (`SceneComponent.K2_SetRelativeRotation` (`self.StaticMesh`) (`KismetMathLibrary.RLerp` (struct) (struct :`Yaw` 90.0) _track) false false)))))))

(event `Close`
  (goto _label :!via `Reverse`))

(fn `UserConstructionScript`)